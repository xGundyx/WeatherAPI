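; Weather player controller that creates the weather HUD and applies received weather data to it and the level's sky.
; Parsed JSON responses fill the display, set sunrise, sunset and time of day on the WeatherTOD actor, and drive skybox cloud cover.
; Failed or invalid responses show display errors.
; It also toggles between display and panel with matching input modes, and converts custom times by GMT offset before applying them to the sun.
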(event Custom|SetCustomTime
  (params (Hour :type Integer) (Minute :type Integer) (PM :type Boolean))
  (bind _returnvalue (Math|DateTime|UTCNow))
  (bind (_year _month _day _hour _minute _second _millisecond) (Math|DateTime|BreakDateTime _returnvalue))
  (Class|WeatherTOD|SetTOD (Variables|Default|GetSun) (+ (Math|DateTime|MakeDateTime _year _month _day Hour Minute _second _millisecond) (Math|Timespan|MakeTimespan 0 (* (Variables|Default|GetGMT) -1)))))

(event EventBeginPlay
  (Utilities|FlowControl|Delay 0.1)
  (bind _returnvalue (UserInterface|CreateWidget "/Game/Weather/UI/WeatherMain.WeatherMain_C" self))
  (UserInterface|Viewport|AddtoViewport _returnvalue 0)
  (Variables|Default|SetHUD _returnvalue)
  (bind _outactors (Actor|GetAllActorsOfClass "/Script/WeatherAPI.WeatherTOD"))
  (Utilities|IsValid (Utilities|Array|Get(acopy) _outactors)
    (:Is%20Valid
      (Variables|Default|SetSun (Utilities|Array|Get(acopy) _outactors)))))

(event EventTick
  (params (DeltaSeconds :type Float%20%28single-precision%29)))

(event EventEventWeatherDataReceived
  (params (Obj :type Play%20Fab%20Json%20Object%20Object%20Reference))
  (bind _returnvalue (Class|PlayFabJsonObject|GetObjectField Obj "main"))
  (bind _returnvalue_2 (Class|PlayFabJsonObject|GetObjectField Obj "wind"))
  (bind _returnvalue_3 (Class|PlayFabJsonObject|GetObjectField Obj "sys"))
  (bind _returnvalue_4 (Class|PlayFabJsonObject|GetStringField Obj "name"))
  (bind _hud (Variables|Default|GetHUD))
  (bind _hud_2 (Variables|Default|GetHUD))
  (bind _hud_3 (Variables|Default|GetHUD))
  (bind _sun (Variables|Default|GetSun))
  (bind _panel (Variables|/Game/Weather/UI/WeatherMain.WeatherMain_C|GetPanel _hud_2))
  (bind _display (Variables|/Game/Weather/UI/WeatherMain.WeatherMain_C|GetDisplay _hud))
  (bind _display_2 (Variables|/Game/Weather/UI/WeatherMain.WeatherMain_C|GetDisplay _hud_3))
  (bind _returnvalue_5 (Widget|IsVisible _display))
  (switch Utilities|FlowControl|Switch|SwitchonERequestError (Utilities|Enum|ByteToEnumERequestError (Math|Conversions|ToByte(Integer) (Math|Float|Floor (Class|PlayFabJsonObject|GetNumberField Obj "code"))))
    (:WEATHER_SUCCESS
      (bind _returnvalue_6 (Class|PlayFabJsonObject|GetObjectArrayField Obj "weather"))
      (for _array_element _returnvalue_6
        (Default|SetMain _display_2 (Class|PlayFabJsonObject|GetStringField _array_element "main") (Class|PlayFabJsonObject|GetStringField _array_element "description")))
      (Default|SetTemp _display_2 (Class|PlayFabJsonObject|GetNumberField _returnvalue "temp") (Class|PlayFabJsonObject|GetNumberField _returnvalue "pressure") (Class|PlayFabJsonObject|GetNumberField _returnvalue "humidity"))
      (Default|SetWind _display_2 (Class|PlayFabJsonObject|GetNumberField _returnvalue_2 "speed") (Class|PlayFabJsonObject|GetNumberField _returnvalue_2 "deg"))
      (bind _returnvalue_7 (Class|WeatherPlayerController|GetUnixTime (Math|Float|Truncate (Class|PlayFabJsonObject|GetNumberField _returnvalue_3 "sunrise"))))
      (bind _returnvalue_8 (Class|WeatherPlayerController|GetUnixTime (Math|Float|Truncate (Class|PlayFabJsonObject|GetNumberField _returnvalue_3 "sunset"))))
      (Default|SetSun _display_2 _returnvalue_8 _returnvalue_7)
      (Class|WeatherTOD|Init _sun _returnvalue_7 _returnvalue_8)
      (Default|SetCity _display_2 _returnvalue_4)
      (Variables|Default|SetCity _returnvalue_4)
      (Variables|Default|SetCountry (Class|PlayFabJsonObject|GetStringField _returnvalue_3 "country"))
      (bind _asbase_weather (Utilities|Casting|CastToBaseWeather (Variables|Default|GetSun)))
      (Variables|/Engine/EngineSky/BP_Sky_Sphere.BP_Sky_Sphere_C|SetTargetClouds (Variables|/Game/Weather/Blueprints/BaseWeather.BaseWeather_C|GetSkyBox _asbase_weather) (/ (Class|PlayFabJsonObject|GetNumberField (Class|PlayFabJsonObject|GetObjectField Obj "clouds") "all") 1e+02))
      (if (Widget|IsVisible _panel)
        (Default|Init _panel))
      (Class|WeatherTOD|SetTOD _sun (Math|DateTime|UTCNow)))
    (:WEATHER_FAIL
      (if _returnvalue_5
        (Default|SetError _display "FAILED TO READ IN WEATHER DATA")))
    (:WEATHER_INVALID
      (if _returnvalue_5
        (Default|SetError _display "WEATHER DATA IS INVALID")))))

(event EventEventOpenPanel
  (bind _self self)
  (bind _hud (Variables|Default|GetHUD))
  (bind _display (Variables|/Game/Weather/UI/WeatherMain.WeatherMain_C|GetDisplay _hud))
  (bind _panel (Variables|/Game/Weather/UI/WeatherMain.WeatherMain_C|GetPanel _hud))
  (if (Widget|IsVisible _display)
    (Widget|SetVisibility _display "Hidden")
    (Widget|SetVisibility _panel "SelfHitTestInvisible")
    (Input|SetInputModeGameandUI _self 0 "DoNotLock" true)
    (Variables|Default|SetbShowMouseCursor true)
    (Default|Init _panel)
    (else
      (Widget|SetVisibility _display "SelfHitTestInvisible")
      (Widget|SetVisibility _panel "Hidden")
      (Input|SetInputModeGameOnly _self)
      (Variables|Default|SetbShowMouseCursor false))))

(event EventEventPanelError
  (params (Msg :type String))
  (bind _hud (Variables|Default|GetHUD))
  (bind _panel (Variables|/Game/Weather/UI/WeatherMain.WeatherMain_C|GetPanel _hud))
  (if (Widget|IsVisible _panel)
    (Default|ShowPanelError _panel Msg)))

(fn ConstructionScript)