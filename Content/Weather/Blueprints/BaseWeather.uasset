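; BaseWeather is a weather base Blueprint that serves as the sky sphere's directional light, keeping the visible sun in step with it.
; On BeginPlay it finds a BP_Sky_Sphere and assigns itself as that sphere's DirectionalLightActor.
; Tick then calls UpdateSunDirection on the sphere every frame, without a validity check.
; The time-of-day update event is empty, and the sun height and cloud logic is unconnected.
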(event EventBeginPlay
  (bind _outactors (Actor|GetAllActorsOfClass "/Engine/EngineSky/BP_Sky_Sphere.BP_Sky_Sphere_C"))
  (for _array_element _outactors
    (Variables|Default|SetSkyBox _array_element))
  (Utilities|IsValid (Variables|Default|GetSkyBox)
    (:Is%20Valid
      (Variables|/Engine/EngineSky/BP_Sky_Sphere.BP_Sky_Sphere_C|SetDirectional%20light%20actor (Variables|Default|GetSkyBox) self))))

(event EventTick
  (params (DeltaSeconds :type Float%20%28single-precision%29))
  (Default|UpdateSunDirection (Variables|Default|GetSkyBox)))

(event EventEventTODUpdated)

(fn ConstructionScript)